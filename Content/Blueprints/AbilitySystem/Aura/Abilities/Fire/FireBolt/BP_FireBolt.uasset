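; BP_FireBolt is the Fire Bolt ability's projectile actor, which can home in on a target.
; On BeginPlay it prints a debug string and starts a looping timer that checks the homing target.
; When the target component is invalid or its owner is dead, it disables homing and clears the timer.
; An unconnected stall check that would play impact effects and destroy the bolt never runs.
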(event Custom|CheckValidEnemyTarget
  (bind _homingtargetcomponent (Variables|/Script/Engine.ProjectileMovementComponent|GetHomingTargetComponent (Variables|Default|GetProjectileMovement))
    (:then
      (bind _returnvalue (Class|CombatInterface|IsDead(Message) (Components|GetOwner _homingtargetcomponent)))
      (if _returnvalue
        (Variables|/Script/Engine.ProjectileMovementComponent|SetbIsHomingProjectile (Variables|Default|GetProjectileMovement) false :!label _label)
        (Utilities|Time|ClearandInvalidateTimerbyHandle (Variables|Default|GetCheckHomingTargetHandle))))
    (:else
      (goto _label))))

(event EventBeginPlay
  (bind _returnvalue (Utilities|Time|SetTimerbyEvent (delegate Custom|CheckValidEnemyTarget) 0.5 true true))
  (Variables|Default|SetCheckHomingTargetHandle _returnvalue)
  (Development|PrintString "Hello"))

(event Collision|EventActorBeginOverlap
  (params (OtherActor :type Actor%20Object%20Reference)))

(event EventTick
  (params (DeltaSeconds :type Float%20%28single-precision%29)))

(fn ConstructionScript)
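; GA_FireBolt is the Gameplay Ability that casts Aura's fire bolt at the location under the mouse.
; After committing, it takes the hit location from the TargetDataUnderMouse task and passes it to the avatar's CombatInterface as the facing target for motion warping.
; It plays the cast montage, spawns projectiles from the weapon socket on the montage's gameplay event, and ends when the montage completes, blends out or is stopped.
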(event Ability|EventActivateAbility
  (Ability|CommitAbility)
  (bind _datahandle (|TargetDataUnderMouse)
    (:ValidData
      (Variables|Default|SetProjectileTargetLocation (.Location (Collision|BreakHitResult (Ability|TargetData|GetHitResultfromTargetData _datahandle))))
      ;[0.02687 0 0.3594 0.5] MotionWarping for BP_AuraCharacter in AM_CastFirebolt
      (bind _ascombat_interface (Utilities|Casting|CastToCombatInterface (Ability|GetAvatarActorfromActorInfo)))
      (Class|CombatInterface|UpdateFacingTarget _ascombat_interface (Variables|Default|GetProjectileTargetLocation))
      (|PlayMontageandWaitProxy "None" "/Game/Assets/Characters/Aura/Animations/Abilities/AM_Cast_FireBolt.AM_Cast_FireBolt" 1.0 "None" false 1.0 0.0 false
        (:then
          (Ability|Tasks|WaitGameplayEvent "(TagName=\"Event.Montage.FireBolt\")" 0
            (:then
              (Class|AuraFireBolt|SpawnProjectiles (Variables|Default|GetProjectileTargetLocation) (GameplayTags|MakeLiteralGameplayTag "(TagName=\"CombatSocket.Weapon\")") true 0.0))))
        (:OnCompleted
          (Ability|EndAbility :!label _label))
        (:OnBlendOut
          (goto _label))
        (:OnInterrupted
          (goto _label))
        (:OnCancelled
          (goto _label))))))
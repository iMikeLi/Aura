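; Enemy melee attack gameplay ability that plays a random tagged attack montage and damages non-friendly players caught by the swing.
; A looping timer keeps the avatar facing its combat target through the CombatInterface until the montage ends.
; The montage's gameplay event triggers a small-radius live-player search at the tag's combat socket, applying damage to each hostile found.
; Montage completion, interruption or cancellation clears the timer and ends the ability.
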(event Ability|EventActivateAbility
  (bind _returnvalue (Ability|GetAvatarActorfromActorInfo))
  (bind _ascombat_interface (Utilities|Casting|CastToCombatInterface (Ability|GetAvatarActorfromActorInfo)))
  (Variables|Default|SetAs%20Combat%20Interface _ascombat_interface)
  (Utilities|FlowControl|Sequence
    (:then_0
      (Utilities|Time|SetTimerbyFunctionName 0 "GetUpdatedEnemyLocation" 0.1 true true))
    (:then_1
      (bind _returnvalue_2 (Class|CombatInterface|GetAttackMontages(Message) (Ability|GetAvatarActorfromActorInfo)))
      (bind _output_get (Variables|Default|SetTaggedMontage (Class|AuraDamageGameplayAbility|GetRandomTaggedMontagefromArray _returnvalue_2)))
      (|PlayMontageandWaitProxy "None" (.Montage (Utilities|Struct|BreakTaggedMontage _output_get)) 1.0 "None" false 1.0 0.0 false
        (:then
          (Ability|Tasks|WaitGameplayEvent (.MontageTag (Utilities|Struct|BreakTaggedMontage _output_get)) 0
            (:EventReceived
              (bind _returnvalue_3 (Class|CombatInterface|GetCombatSocketLocation(Message) _returnvalue (.MontageTag (Utilities|Struct|BreakTaggedMontage _output_get))))
              (bind _outoverlappingactors (Class|AuraAbilitySystemLibrary|GetLivePlayersWithinRadius self (Utilities|Array|MakeArray _returnvalue) 45.0 _returnvalue_3))
              (for _array_element _outoverlappingactors
                (if (Class|AuraAbilitySystemLibrary|IsNotFriend (Ability|GetAvatarActorfromActorInfo) _array_element)
                  (Class|AuraDamageGameplayAbility|CauseDamage _array_element))))))
        (:OnCompleted
          (Utilities|Time|ClearTimerbyFunctionName 0 "GetUpdatedEnemyLocation" :!label _label)
          (Ability|EndAbility))
        (:OnInterrupted
          (goto _label))
        (:OnCancelled
          (goto _label))))))

(event Ability|EventOnEndAbility
  (params (bWasCancelled :type Boolean)))

(fn GetUpdatedEnemyLocation
  (bind _returnvalue (Class|EnemyInterface|GetCombatTarget(Message) (Ability|GetAvatarActorfromActorInfo)))
  (Utilities|IsValid _returnvalue
    (:Is%20Valid
      (Class|CombatInterface|UpdateFacingTarget (Variables|Default|GetAs%20Combat%20Interface) (Transformation|GetActorLocation _returnvalue)))))
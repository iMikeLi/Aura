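; Enemy ranged attack gameplay ability that fires a projectile at the avatar's combat target.
; On activation it plays a random tagged attack montage while a looping timer keeps updating the avatar's facing target to the combat target's location.
; The montage's gameplay event spawns the projectile from the tagged socket, then clears the timer and ends the ability without stopping the montage.
; Montage completion, interruption or cancellation also clears the timer and ends the ability.
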(event Ability|EventActivateAbility
  (Utilities|FlowControl|Sequence
    (:then_0
      (Utilities|Time|SetTimerbyFunctionName 0 "GetUpdatedEnemyLocation" 0.1 true true))
    (:then_1
      (bind _returnvalue (Class|CombatInterface|GetAttackMontages(Message) (Ability|GetAvatarActorfromActorInfo)))
      (bind _output_get (Variables|Default|SetTaggedMontage (Class|AuraDamageGameplayAbility|GetRandomTaggedMontagefromArray _returnvalue)))
      (|PlayMontageandWaitProxy "None" (.Montage (Utilities|Struct|BreakTaggedMontage _output_get)) 1.0 "None" false 1.0 0.0 false
        (:then
          (Ability|Tasks|WaitGameplayEvent (.MontageTag (Utilities|Struct|BreakTaggedMontage _output_get)) 0 true
            (:EventReceived
              (bind _returnvalue_2 (Class|EnemyInterface|GetCombatTarget(Message) (Ability|GetAvatarActorfromActorInfo)))
              (Class|AuraProjectileSpell|SpawnProjectile (Transformation|GetActorLocation _returnvalue_2) (.SocketTag (Utilities|Struct|BreakTaggedMontage _output_get)) (Variables|Default|GetShouldOverride%20Pitch) (Variables|Default|GetPitchOverride))
              (Utilities|Time|ClearTimerbyFunctionName 0 "GetUpdatedEnemyLocation")
              (Ability|EndAbility))))
        (:OnCompleted
          (Utilities|Time|ClearTimerbyFunctionName 0 "GetUpdatedEnemyLocation" :!label _label)
          (Ability|EndAbility))
        (:OnInterrupted
          (goto _label))
        (:OnCancelled
          (goto _label))))))

(event Ability|EventOnEndAbility
  (params (bWasCancelled :type Boolean)))

(fn GetUpdatedEnemyLocation
  (bind _returnvalue (Ability|GetAvatarActorfromActorInfo))
  (bind _returnvalue_2 (Class|EnemyInterface|GetCombatTarget(Message) _returnvalue))
  (Utilities|IsValid _returnvalue_2
    (:Is%20Valid
      (Class|CombatInterface|UpdateFacingTarget(Message) _returnvalue (Transformation|GetActorLocation _returnvalue_2)))))